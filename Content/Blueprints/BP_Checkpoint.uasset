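; BP_Checkpoint is a checkpoint trigger that saves the custom third-person character's progress when it overlaps the Cylinder component.
; The Visible variable sets the cylinder's visibility on BeginPlay and gates the activation bell sound.
; A Playonce flag limits that sound and the switch to a green glass material to the first overlap, while SaveCheckpoint is called on the character every time.
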(event OnComponentBeginOverlap(Cylinder)
  (params (OverlappedComponent :type Primitive%20Component%20Object%20Reference) (OtherActor :type Actor%20Object%20Reference) (OtherComp :type Primitive%20Component%20Object%20Reference) (OtherBodyIndex :type Integer) (bFromSweep :type Boolean) (SweepResult :type Hit%20Result%20Structure%20%28by%20ref%29))
  (bind _asbp_third_person_character_custom (Utilities|Casting|CastToBP_ThirdPersonCharacterCustom OtherActor))
  (if (Variables|Default|Getplayonce)
    _
    (else
      (if (Variables|Default|GetVisible)
        (Audio|PlaySound2D "/Game/Audio/FX/BellSpoon.BellSpoon" 2.0 1.0 0.0 0 0))
      (Variables|Default|Setplayonce true)
      (Rendering|Material|SetMaterial (Variables|Default|GetCylinder) 0 "/Game/Materials/Materials/Glass/MI_FutigerGlass_Green.MI_FutigerGlass_Green")))
  (Default|SaveCheckpoint _asbp_third_person_character_custom))

(event EventBeginPlay
  (Rendering|SetVisibility (Variables|Default|GetCylinder) (Variables|Default|GetVisible) false))

(event Collision|EventActorBeginOverlap
  (params (OtherActor :type Actor%20Object%20Reference)))

(event EventTick
  (params (DeltaSeconds :type Float%20%28single-precision%29)))

(fn ConstructionScript)