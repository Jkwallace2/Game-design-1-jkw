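; Rotating door Blueprint that swings its static mesh open on actor overlap, then closes it automatically.
; The Opendoor timeline drives relative yaw toward -90 degrees and also plays on BeginPlay, without the opening sound.
; On finishing, it toggles IsOpen, reversing after a short delay or playing the close sound once shut.
; Open plays the opening sound and timeline only while IsOpen is false.
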(event Custom|Open
  (bind _staticmeshcomponent (Variables|Debug|GetStaticMeshComponent))
  (bind _returnvalue (Transformation|GetWorldLocation _staticmeshcomponent))
  (if (not (Variables|Default|GetIsOpen))
    (Audio|PlaySoundatLocation "/Game/Audio/FX/DoorOpen.DoorOpen" _returnvalue "0, 0, 0" 1.0 1.0 0.0 0 0 0 0)
    (bind _newtrack_1 (Timeline|Opendoor Play)
      (:Update
        (Transformation|SetRelativeRotation (Variables|Debug|GetStaticMeshComponent) (Math|Rotator|MakeRotator 0.0 0.0 (* _newtrack_1 -9e+01)) false false))
      (:Finished
        (if (Variables|Default|GetIsOpen)
          (Audio|PlaySoundatLocation "/Game/Audio/FX/DoorClose.DoorClose" _returnvalue "0, 0, 0" 1.0 1.0 0.0 0 0 0 0)
          (Variables|Default|SetIsOpen false)
          (else
            (Variables|Default|SetIsOpen true)
            (Utilities|FlowControl|Delay 0.2)
            (Timeline|Opendoor ReverseFromEnd)))))))

(event EventBeginPlay
  (bind _newtrack_1 (Timeline|Opendoor Play)
    (:Update
      (Transformation|SetRelativeRotation (Variables|Debug|GetStaticMeshComponent) (Math|Rotator|MakeRotator 0.0 0.0 (* _newtrack_1 -9e+01)) false false))
    (:Finished
      (if (Variables|Default|GetIsOpen)
        (Audio|PlaySoundatLocation "/Game/Audio/FX/DoorClose.DoorClose" (Transformation|GetWorldLocation (Variables|Debug|GetStaticMeshComponent)) "0, 0, 0" 1.0 1.0 0.0 0 0 0 0)
        (Variables|Default|SetIsOpen false)
        (else
          (Variables|Default|SetIsOpen true)
          (Utilities|FlowControl|Delay 0.2)
          (Timeline|Opendoor ReverseFromEnd))))))

(event Collision|EventActorBeginOverlap
  (params (OtherActor :type Actor%20Object%20Reference))
  (CallFunction|Open))

(event EventTick
  (params (DeltaSeconds :type Float%20%28single-precision%29)))

(fn ConstructionScript)