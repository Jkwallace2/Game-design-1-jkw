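; BP_CubeEnd is an end-piece cube that captures a BP_ToyBall and swaps in a lit ImpBall.
; BallSensor overlaps play a Timeline forward and in reverse, moving the cube, dropper and plane with a snare cue on activation.
; BallInterior overlap stores the ball and latches KillMode, blocking further activation.
; When the Timeline finishes in KillMode, it kills the ball, plays a rimshot and enables ImpBall's visibility, collision and light.
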(event OnComponentBeginOverlap(BallSensor)
  (params (OverlappedComponent :type Primitive%20Component%20Object%20Reference) (OtherActor :type Actor%20Object%20Reference) (OtherComp :type Primitive%20Component%20Object%20Reference) (OtherBodyIndex :type Integer) (bFromSweep :type Boolean) (SweepResult :type Hit%20Result%20Structure%20%28by%20ref%29))
  (Utilities|Casting|CastToBP_ToyBall OtherActor)
  (CallFunction|Activate))

(event OnComponentEndOverlap(BallSensor)
  (params (OverlappedComponent :type Primitive%20Component%20Object%20Reference) (OtherActor :type Actor%20Object%20Reference) (OtherComp :type Primitive%20Component%20Object%20Reference) (OtherBodyIndex :type Integer))
  (Utilities|Casting|CastToBP_ToyBall OtherActor)
  (CallFunction|Deactivate))

(event OnComponentBeginOverlap(BallInterior)
  (params (OverlappedComponent :type Primitive%20Component%20Object%20Reference) (OtherActor :type Actor%20Object%20Reference) (OtherComp :type Primitive%20Component%20Object%20Reference) (OtherBodyIndex :type Integer) (bFromSweep :type Boolean) (SweepResult :type Hit%20Result%20Structure%20%28by%20ref%29))
  (bind _asbp_toy_ball (Utilities|Casting|CastToBP_ToyBall OtherActor))
  (Variables|Default|SetTarget _asbp_toy_ball)
  (Variables|Default|SetKillMode true))

(event Custom|Activate
  (bind _impball (Variables|Default|GetImpBall))
  (if (not (Variables|Default|GetKillMode))
    (Audio|PlaySoundatLocation "/Game/LevelPrototyping/Audio/DrumShots/Cues/Amen_Snare_Low_FC_164_Cue.Amen_Snare_Low_FC_164_Cue" (Transformation|GetWorldLocation (Variables|Default|GetDefaultSceneRoot)) "0, 0, 0" 1.0 1.0 0.0 0 0 0 0)
    (bind _newtrack_1 (Timeline|Timeline Play)
      (:Update
        (Transformation|SetRelativeRotation (Variables|Default|GetSM_Cubeend_Dropper) (Math|Rotator|MakeRotator 0.0 (* _newtrack_1 3e+01) 0.0) false false)
        (Transformation|SetRelativeLocation (Variables|Default|GetSM_Cubeend) (Math|Vector|MakeVector 0.0 0.0 (* _newtrack_1 8e+01)) false false)
        (Transformation|SetRelativeLocation (Variables|Default|GetPlane) (Math|Vector|MakeVector 0.0 0.0 (+ (* _newtrack_1 -25.0) -5e+01)) false false))
      (:Finished
        (if (Variables|Default|GetKillMode)
          (Default|CommitDie (stale OnComponentBeginOverlap(BallInterior) _asbp_toy_ball))
          (Audio|PlaySoundatLocation "/Game/LevelPrototyping/Audio/DrumShots/Cues/Rimshot_Spring_WD_Cue.Rimshot_Spring_WD_Cue" (Transformation|GetWorldLocation (Variables|Default|GetDefaultSceneRoot)) "0, 0, 0" 1.0 1.0 0.0 0 0 0 0)
          (Rendering|SetVisibility _impball true false)
          (Rendering|Components|Light|SetIntensity (Variables|Default|GetPointLight) 8e+02)
          (Collision|SetCollisionEnabled _impball "QueryAndPhysics"))))))

(event Custom|Deactivate
  (bind _impball (Variables|Default|GetImpBall))
  (bind _newtrack_1 (Timeline|Timeline Reverse)
    (:Update
      (Transformation|SetRelativeRotation (Variables|Default|GetSM_Cubeend_Dropper) (Math|Rotator|MakeRotator 0.0 (* _newtrack_1 3e+01) 0.0) false false)
      (Transformation|SetRelativeLocation (Variables|Default|GetSM_Cubeend) (Math|Vector|MakeVector 0.0 0.0 (* _newtrack_1 8e+01)) false false)
      (Transformation|SetRelativeLocation (Variables|Default|GetPlane) (Math|Vector|MakeVector 0.0 0.0 (+ (* _newtrack_1 -25.0) -5e+01)) false false))
    (:Finished
      (if (Variables|Default|GetKillMode)
        (Default|CommitDie (stale OnComponentBeginOverlap(BallInterior) _asbp_toy_ball))
        (Audio|PlaySoundatLocation "/Game/LevelPrototyping/Audio/DrumShots/Cues/Rimshot_Spring_WD_Cue.Rimshot_Spring_WD_Cue" (Transformation|GetWorldLocation (Variables|Default|GetDefaultSceneRoot)) "0, 0, 0" 1.0 1.0 0.0 0 0 0 0)
        (Rendering|SetVisibility _impball true false)
        (Rendering|Components|Light|SetIntensity (Variables|Default|GetPointLight) 8e+02)
        (Collision|SetCollisionEnabled _impball "QueryAndPhysics")))))

(event EventBeginPlay)

(event Collision|EventActorBeginOverlap
  (params (OtherActor :type Actor%20Object%20Reference)))

(event EventTick
  (params (DeltaSeconds :type Float%20%28single-precision%29)))

(fn ConstructionScript
  (Variables|Default|SetKillMode false)
  (Rendering|SetVisibility (Variables|Default|GetImpBall) false false)
  (Rendering|Components|Light|SetIntensity (Variables|Default|GetPointLight) 0.0)
  (Collision|SetCollisionEnabled (Variables|Default|GetImpBall) "NoCollision"))