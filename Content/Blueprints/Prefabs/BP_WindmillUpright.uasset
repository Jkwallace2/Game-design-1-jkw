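; Upright windmill prefab whose blade mesh spins continuously for decoration.
; On BeginPlay it picks a random starting angle and spin speed, so separate instances rotate out of step.
; Each Tick it sets the blade's relative pitch from game time multiplied by that speed, plus the offset.
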(event EventBeginPlay
  (bind _output_get (Variables|Default|SetOffset (Math|Random|RandomIntegerinRange 0 180)))
  (Variables|Default|Setspeed (Math|Random|RandomFloatinRange 1e+01 15.0)))

(event Collision|EventActorBeginOverlap
  (params (OtherActor :type Actor%20Object%20Reference)))

(event EventTick
  (params (DeltaSeconds :type Float%20%28single-precision%29))
  (Transformation|SetRelativeRotation (Variables|Default|GetSM_Windmill_Blade) (Math|Rotator|MakeRotator 0.0 (+ (* (Utilities|Time|GetTimeSeconds) (Variables|Default|Getspeed)) (stale EventBeginPlay _output_get)) 0.0) false false))

(fn ConstructionScript)