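; BP_ToyBall is a puzzle-element physics ball with sound driven by its motion.
; A per-tick downward trace switches between ground drag audio, with filter and pitch scaled by angular speed and Htz, and an airborne ring.
; Strong hits play open or closed impact sounds by impulse direction, scaled by force.
; Construction applies the configurable mesh and sounds, and CommitDie destroys the ball.
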(event Custom|CommitDie
  (Development|PrintString "Shere deleated")
  (Actor|DestroyActor))

(event EventBeginPlay)

(event Collision|EventActorBeginOverlap
  (params (OtherActor :type Actor%20Object%20Reference)))

(event EventTick
  (params (DeltaSeconds :type Float%20%28single-precision%29))
  (bind _collision (Variables|Default|GetCollision))
  (bind _collision_2 (Variables|Default|GetCollision))
  (bind _htz (Variables|Default|GetHtz))
  (bind _drag (Variables|Default|GetDrag))
  (bind _drag_2 (Variables|Default|GetDrag))
  (bind _ring (Variables|Default|GetRing))
  (bind _returnvalue (Transformation|GetWorldLocation _collision_2))
  (bind _returnvalue_2 (Physics|GetPhysicsAngularVelocityinDegrees _collision "None"))
  (bind _returnvalue_3 (/ 6e+01 _htz))
  (bind (_x _y _z) (Math|Vector|BreakVector _returnvalue))
  (bind _returnvalue_4 (Math|Float|Power (.z _returnvalue_2) 2.0))
  (bind _returnvalue_5 (Math|Float|Power (.x _returnvalue_2) 2.0))
  (bind _returnvalue_6 (Math|Float|Power (.y _returnvalue_2) 2.0))
  (bind _returnvalue_7 (+ _returnvalue_5 _returnvalue_6 _returnvalue_4))
  (bind _returnvalue_8 (Math|Float|Sqrt _returnvalue_7))
  (bind _returnvalue_9 (Class|KismetSystemLibrary|LineTraceSinglebyProfile _returnvalue (Math|Vector|MakeVector _x _y (- _z 6e+01)) "BlockAllDynamic" false 0 "None" true))
  ;[1 1 1] true = touching ground
  (if _returnvalue_9
    (Variables|Default|SetSoundRing false)
    (Audio|Components|Audio|Stop _ring)
    (Audio|Components|Audio|SetVolumeMultiplier (Variables|Default|GetDrag) (Variables|Default|GetDrag%20volume) :!class /Script/Engine.AudioComponent)
    (Audio|Components|Audio|SetLowPassFilterFrequency _drag (Math|Float|Power (* (/ _returnvalue_8 2e+01) _returnvalue_3) 2.0) :!class /Script/Engine.AudioComponent)
    (if (Variables|Default|GetSpeedAffectPitch)
      (Audio|Components|Audio|SetPitchMultiplier _drag (* (/ _returnvalue_8 3.6e+02) _returnvalue_3))
      (else
        (Audio|Components|Audio|SetPitchMultiplier _drag (Math|Float|Clamp(Float) (* _returnvalue_8 _returnvalue_3) 0.0 (Variables|Default|GetPitchOffset)))))
    (else
      (if (!= (Variables|Default|GetSoundRing) true)
        (Audio|Components|Audio|SetVolumeMultiplier _ring 1.0 :!class /Script/Engine.AudioComponent)
        (Audio|Components|Audio|SetPitchMultiplier _ring (Variables|Default|GetPitchOffset))
        (Audio|Components|Audio|Play _ring 0.0))
      (Variables|Default|SetSoundRing true)
      (if (Variables|Default|GetContinuouslooping?)
        (Audio|Components|Audio|SetVolumeMultiplier _drag_2 0.1 :!class /Script/Engine.AudioComponent)
        (else
          (Audio|Components|Audio|SetVolumeMultiplier _drag_2 0.0 :!class /Script/Engine.AudioComponent))))))

(event Collision|EventHit
  (params (MyComp :type Primitive%20Component%20Object%20Reference) (Other :type Actor%20Object%20Reference) (OtherComp :type Primitive%20Component%20Object%20Reference) (bSelfMoved :type Boolean) (HitLocation :type Vector :default "0, 0, 0") (HitNormal :type Vector :default "0, 0, 0") (NormalImpulse :type Vector :default "0, 0, 0") (Hit :type Hit%20Result%20Structure%20%28by%20ref%29))
  (bind _returnvalue (Math|Float|Absolute(Float) (.y NormalImpulse)))
  (bind _returnvalue_2 (Math|Float|Absolute(Float) (.z NormalImpulse)))
  (bind _returnvalue_3 (Math|Float|Absolute(Float) (.x NormalImpulse)))
  (bind _ring (Variables|Default|GetRing))
  (bind _pitchoffset (Variables|Default|GetPitchOffset))
  (bind _returnvalue_4 (+ _returnvalue_3 _returnvalue))
  (bind _returnvalue_5 (+ _returnvalue_4 _returnvalue_2))
  (bind _returnvalue_6 (/ _returnvalue_5 3.0))
  (bind _returnvalue_7 (* _returnvalue_6 5e-05))
  (bind _returnvalue_8 (Math|Float|Clamp(Float) _returnvalue_7 0.0 3.0))
  (bind _returnvalue_9 (Math|Float|MapRangeUnclamped _returnvalue_7 1.0 1e+01 1.0 1.1))
  (bind _returnvalue_10 (* _returnvalue_9 _pitchoffset))
  (Utilities|FlowControl|DelayUntilNextTick)
  (Audio|Components|Audio|Stop (Variables|Default|GetRing))
  (if (> _returnvalue_6 1.5e+03)
    (if (> (.z NormalImpulse) 0.01)
      (Audio|PlaySoundatLocation (Variables|Default|GetSND_Impact_Open) HitLocation "0, 0, 0" _returnvalue_8 _returnvalue_10 0.0 0 0 0 0)
      (else
        (Audio|PlaySoundatLocation (Variables|Default|GetSND_Impact_Closed) HitLocation "0, 0, 0" _returnvalue_8 _returnvalue_10 0.0 0 0 0 0)))
    (if (Variables|Default|GetSoundRing)
      (Development|PrintString "RING")
      (Audio|Components|Audio|SetPitchMultiplier _ring (Variables|Default|GetPitchOffset))
      (Audio|Components|Audio|SetVolumeMultiplier _ring 1.0 :!class /Script/Engine.AudioComponent)
      (Audio|Components|Audio|Play _ring 0.0))))

(fn ConstructionScript
  (bind _mesh (Variables|Default|GetMesh))
  (Audio|Components|Audio|SetSound (Variables|Default|GetDrag) (Variables|Default|GetSND_Drag))
  (Audio|Components|Audio|SetSound (Variables|Default|GetRing) (Variables|Default|GetSND_Ring))
  (Audio|Components|Audio|SetLowPassFilterEnabled (Variables|Default|GetDrag) (Variables|Default|GetAllowLowPass?) :!class /Script/Engine.AudioComponent)
  (Components|StaticMesh|SetStaticMesh _mesh (Variables|Default|GetBallMesh))
  (Collision|SetCollisionEnabled _mesh "NoCollision"))

(fn VelocityasFloat
  (params (Target :type Scene%20Component%20Object%20Reference))
  (bind _returnvalue (Transformation|GetComponentVelocity Target))
  (return (/ (+ (Math|Float|Absolute(Float) (.x _returnvalue)) (Math|Float|Absolute(Float) (.y _returnvalue)) (Math|Float|Absolute(Float) (.z _returnvalue))) 3.0)))