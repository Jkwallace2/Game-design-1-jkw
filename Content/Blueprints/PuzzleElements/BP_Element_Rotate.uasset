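; Puzzle element that pitches its root component by up to -90 degrees via a timeline when activated, playing a door-open sound at the cube.
; A DoOnce blocks repeat activation until Reset.
; Reset uses a second timeline to lerp from the current transform back to the original cached in construction and BeginPlay, then re-arms the DoOnce when finished.
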(event EventBeginPlay
  (Development|SetHiddeninGame (Variables|Default|GetCube) false false)
  (Variables|Default|SetOriginalTransform (Transformation|GetRelativeTransform (Variables|Default|GetDefaultSceneRoot))))

(event Collision|EventActorBeginOverlap
  (params (OtherActor :type Actor%20Object%20Reference)))

(event EventTick
  (params (DeltaSeconds :type Float%20%28single-precision%29))
  (|CallParentFunction DeltaSeconds) ; This node is disabled and will not be called.\nDrag off pins to build functionality.
)

(event EventActivate
  (Utilities|FlowControl|DoOnce false
    (:Completed
      (Audio|PlaySoundatLocation "/Game/Audio/FX/DoorOpen.DoorOpen" (Transformation|GetWorldLocation (Variables|Default|GetCube)) "0, 0, 0" 1.0 1.0 0.0 0 0 0 0)
      (bind _newtrack_1 (Timeline|Timeline PlayFromStart)
        (:Update
          (Transformation|SetRelativeRotation (Variables|Default|GetDefaultSceneRoot) (Math|Rotator|MakeRotator 0.0 (* _newtrack_1 -9e+01) 0.0) false false))))))

(event EventReset
  (Variables|Default|SetCurentTransform (Transformation|GetRelativeTransform (Variables|Default|GetDefaultSceneRoot)))
  (bind _floattrack (Timeline|Timeline_0 PlayFromStart)
    (:Update
      (Transformation|SetRelativeTransform (Variables|Default|GetDefaultSceneRoot) (Math|Transform|Lerp(Transform) (Variables|Default|GetCurentTransform) (Variables|Default|GetOriginalTransform) _floattrack) false false))
    (:Finished
      (Utilities|FlowControl|DoOnce false) ; enters at Reset
    )))

(fn ConstructionScript
  (Rendering|SetVisibility (Variables|Default|GetCube) true false)
  (Variables|Default|SetOriginalTransform (Transformation|GetRelativeTransform (Variables|Default|GetDefaultSceneRoot))))