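; Puzzle-element ball spawner that, when activated, spawns a BP_ToyBall at its root and animates a pair of arm meshes.
; Spawning hides the preview Sphere and is capped by MaxBalls, with a count that only resets in the construction script.
; Two chained timelines drive the arms' pitch with a short delay between them, and an Activated flag blocks retriggering until the second finishes.
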(event Custom|Activate
  (bind _sm_arm_ld1 (Variables|Default|GetSM_Arm_LD1))
  (bind _sm_arm_ld (Variables|Default|GetSM_Arm_LD))
  (bind _relativerotation (Variables|/Script/Engine.SceneComponent|GetRelativeRotation _sm_arm_ld1))
  (bind _relativerotation_2 (Variables|/Script/Engine.SceneComponent|GetRelativeRotation _sm_arm_ld))
  (if (not (Variables|Default|GetActivated))
    (Variables|Default|SetActivated true)
    (CallFunction|SpawnBall)
    (bind _newtrack_1 (Timeline|Timeline PlayFromStart)
      (:Update
        (Transformation|SetRelativeRotation _sm_arm_ld (Math|Rotator|MakeRotator (.roll _relativerotation_2) (* _newtrack_1 8e+01) (.yaw _relativerotation_2)) false false)
        (Transformation|SetRelativeRotation _sm_arm_ld1 (Math|Rotator|MakeRotator (.roll _relativerotation) (* _newtrack_1 8e+01) (.yaw _relativerotation)) false false))
      (:Finished
        (Utilities|FlowControl|Delay 0.1)
        (bind _newtrack_1_2 (Timeline|Timeline_0 PlayFromStart)
          (:Update
            (Transformation|SetRelativeRotation _sm_arm_ld1 (Math|Rotator|MakeRotator (.roll _relativerotation) (* _newtrack_1_2 8e+01) (.yaw _relativerotation)) false false)
            (Transformation|SetRelativeRotation _sm_arm_ld (Math|Rotator|MakeRotator (.roll _relativerotation_2) (* _newtrack_1_2 8e+01) (.yaw _relativerotation_2)) false false))
          (:Finished
            (Variables|Default|SetActivated false)))))))

(event Custom|SpawnBall
  (if (< (Variables|Default|GetMy%20Balls) (Variables|Default|GetMax%20Balls))
    (Variables|Default|SetMy%20Balls (+ (Variables|Default|GetMy%20Balls) 1))
    (Rendering|SetVisibility (Variables|Default|GetSphere) false false)
    (Game|SpawnActorfromClass "/Game/Blueprints/PuzzleElements/BP_ToyBall.BP_ToyBall_C" (Math|Conversions|ToTransform(Vector) (Transformation|GetWorldLocation (Variables|Default|GetDefaultSceneRoot))) "Undefined" "MultiplyWithRoot" 0 0)
    (Development|PrintText "Ball Spawned!")))

(event EventBeginPlay)

(event Collision|EventActorBeginOverlap
  (params (OtherActor :type Actor%20Object%20Reference)))

(event EventTick
  (params (DeltaSeconds :type Float%20%28single-precision%29)))

(fn ConstructionScript
  (Variables|Default|SetMy%20Balls 0)
  (Rendering|SetVisibility (Variables|Default|GetSphere) true false))