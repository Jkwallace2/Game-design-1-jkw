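; BP_Coin_Phys is a physics-capable coin pickup that flies into the player and vanishes when touched.
; A one-shot capsule overlap with BP_ThirdPersonCharacterCustom disables physics and collision, plays a coin sound and starts a timeline.
; The timeline lerps the coin toward the character's live location while shrinking it from its construction-time scale, then destroys the actor.
; A separate OnSpawn event plays an impact sound at a supplied pitch.
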(event OnComponentBeginOverlap(Capsule)
  (params (OverlappedComponent :type Primitive%20Component%20Object%20Reference) (OtherActor :type Actor%20Object%20Reference) (OtherComp :type Primitive%20Component%20Object%20Reference) (OtherBodyIndex :type Integer) (bFromSweep :type Boolean) (SweepResult :type Hit%20Result%20Structure%20%28by%20ref%29))
  (bind _coin (Variables|Default|GetCoin))
  (Utilities|FlowControl|DoOnce false :!label _label
    (:Completed
      (bind _asbp_third_person_character_custom (Utilities|Casting|CastToBP_ThirdPersonCharacterCustom OtherActor)
        (:then
          (Physics|SetSimulatePhysics (Variables|Default|GetCoin) false)
          (Collision|SetCollisionEnabled (Variables|Default|GetCapsule) "NoCollision")
          (Audio|PlaySoundatLocation "/Game/Audio/FX/coin.coin" (Transformation|GetActorLocation _asbp_third_person_character_custom) "0, 0, 0" 0.5 1.0 0.0 0 0 0 0)
          (bind _newtrack_1 (Timeline|Timeline_0 PlayFromStart)
            (:Update
              (Transformation|SetWorldLocation _coin (Math|Vector|Lerp(Vector) (Transformation|GetWorldLocation (Variables|Default|GetCoin)) (Transformation|GetActorLocation _asbp_third_person_character_custom) _newtrack_1) false false)
              (Transformation|SetRelativeScale3D _coin (* (Math|Conversions|ToVector(Float) (- 1.0 _newtrack_1)) (Variables|Default|GetRelative%20Scale%203D))))
            (:Finished
              (Actor|DestroyActor))))
        (:CastFailed
          (goto _label Reset))))))

(event Custom|On%20Spawn
  (params (PitchOffset :type Float%20%28double-precision%29))
  (Audio|PlaySoundatLocation "/Game/Audio/Physics/Crystal_ImpactOpen.Crystal_ImpactOpen" "0, 0, 0" "0, 0, 0" 0.5 PitchOffset 0.0 0 0 0 0))

(fn ConstructionScript
  (Variables|Default|SetRelative%20Scale%203D (Variables|/Script/Engine.SceneComponent|GetRelativeScale3D (Variables|Default|GetCoin))))