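; Puzzle end kiosk that accepts a toy ball of its configured color and activates its linked Target.
; The construction script themes button, sphere and light by color, hides the sphere and caches its resting position.
; On box overlap, a DoOnce gate resets for non-matching actors; a match kills the ball and reveals the stand-in sphere.
; A timeline lerps the sphere into place, then plays a bell and activates Target.
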(event OnComponentBeginOverlap(Box)
  (params (OverlappedComponent :type Primitive%20Component%20Object%20Reference) (OtherActor :type Actor%20Object%20Reference) (OtherComp :type Primitive%20Component%20Object%20Reference) (OtherBodyIndex :type Integer) (bFromSweep :type Boolean) (SweepResult :type Hit%20Result%20Structure%20%28by%20ref%29))
  (bind _target (Variables|Default|GetTarget))
  (bind _sphere (Variables|Default|GetSphere))
  (Utilities|FlowControl|DoOnce false :!label _label
    (:Completed
      (switch Utilities|FlowControl|Switch|SwitchonEnum_Colors (Variables|Default|GetColors)
        (:NewEnumerator0
          (bind _asbp_toy_ball_red (Utilities|Casting|CastToBP_ToyBall_red OtherActor)
            (:then
              (Variables|Default|SetLerpLocation (Transformation|GetWorldLocation (Variables|/Game/Blueprints/PuzzleElements/BP_ToyBall.BP_ToyBall_C|GetCollision _asbp_toy_ball_red)))
              (Default|CommitDie _asbp_toy_ball_red))
            (:CastFailed
              (goto _label Reset))))
        (:NewEnumerator1
          (bind _asbp_toy_ball_green (Utilities|Casting|CastToBP_ToyBall_Green OtherActor)
            (:then
              (Variables|Default|SetLerpLocation (Transformation|GetWorldLocation (Variables|/Game/Blueprints/PuzzleElements/BP_ToyBall.BP_ToyBall_C|GetCollision _asbp_toy_ball_green)))
              (Default|CommitDie _asbp_toy_ball_green))
            (:CastFailed
              (goto _label Reset))))
        (:NewEnumerator2
          (bind _asbp_toy_ball_blue (Utilities|Casting|CastToBP_ToyBall_Blue OtherActor)
            (:then
              (Variables|Default|SetLerpLocation (Transformation|GetWorldLocation (Variables|/Game/Blueprints/PuzzleElements/BP_ToyBall.BP_ToyBall_C|GetCollision _asbp_toy_ball_blue)))
              (Default|CommitDie _asbp_toy_ball_blue))
            (:CastFailed
              (goto _label Reset))))
        (:NewEnumerator3
          (bind _asbp_toy_ball_yellow (Utilities|Casting|CastToBP_ToyBall_yellow OtherActor)
            (:then
              (Variables|Default|SetLerpLocation (Transformation|GetWorldLocation (Variables|/Game/Blueprints/PuzzleElements/BP_ToyBall.BP_ToyBall_C|GetCollision _asbp_toy_ball_yellow)))
              (Default|CommitDie _asbp_toy_ball_yellow))
            (:CastFailed
              (goto _label Reset))))
        (:NewEnumerator4
          (bind _asbp_toy_ball_black (Utilities|Casting|CastToBP_ToyBall_Black OtherActor)
            (:then
              (Variables|Default|SetLerpLocation (Transformation|GetWorldLocation (Variables|/Game/Blueprints/PuzzleElements/BP_ToyBall.BP_ToyBall_C|GetCollision _asbp_toy_ball_black)))
              (Default|CommitDie _asbp_toy_ball_black)
              (Variables|Default|SetShowLight false))
            (:CastFailed
              (goto _label Reset)))))
      (Rendering|SetVisibility _sphere true false)
      (Collision|SetCollisionEnabled _sphere "QueryAndPhysics")
      (if (Variables|Default|GetShowLight)
        (Rendering|ToggleVisibility (Variables|Default|GetPointLight) false)
        (bind _newtrack_0 (Timeline|Timeline Play)
          (:Update
            (Transformation|SetWorldLocation (Variables|Default|GetSphere) (Math|Vector|Lerp(Vector) (Variables|Default|GetLerpLocation) (Variables|Default|GetMyLocation) _newtrack_0) false false))
          (:Finished
            (Audio|PlaySoundatLocation "/Game/Audio/FX/BellSpoon.BellSpoon" (Transformation|GetWorldLocation (Variables|Default|GetDefaultSceneRoot)) "0, 0, 0" 1.0 1.0 0.0 0 0 0 0)
            (if (Utilities|IsValid _target)
              (Default|Activate _target))))
        (else
          (Timeline|Timeline Play))))))

(event EventBeginPlay
  (|CallParentFunction) ; This node is disabled and will not be called.\nDrag off pins to build functionality.
)

(event EventTick
  (params (DeltaSeconds :type Float%20%28single-precision%29))
  (|CallParentFunction DeltaSeconds) ; This node is disabled and will not be called.\nDrag off pins to build functionality.
)

(fn ConstructionScript
  (bind _button (Variables|Default|GetButton))
  (bind _sphere (Variables|Default|GetSphere))
  (bind _pointlight (Variables|Default|GetPointLight))
  (Collision|SetCollisionEnabled (Variables|Default|GetButton) "PhysicsOnly")
  (Rendering|SetVisibility (Variables|Default|GetSphere) false false)
  (Variables|Default|SetLookForBall true)
  (Variables|Default|SetDoColorToggle false)
  (Collision|SetCollisionEnabled (Variables|Default|GetSphere) "NoCollision")
  (Rendering|ToggleVisibility (Variables|Default|GetPointLight) false)
  (Variables|Default|SetMyLocation (Transformation|GetWorldLocation (Variables|Default|GetSphere)))
  (switch Utilities|FlowControl|Switch|SwitchonEnum_Colors (Variables|Default|GetColors)
    (:NewEnumerator0
      (Rendering|Material|SetMaterial _button 0 "/Game/Materials/Materials/Coins/Mi_Coin_Red.Mi_Coin_Red")
      (Rendering|Material|SetMaterial _sphere 0 "/Game/Materials/Materials/Glass/MI_FutigerGlass_Red.MI_FutigerGlass_Red")
      (Rendering|Components|Light|SetLightColor _pointlight "(R=1.000000,G=0.298039,B=0.215686,A=1.000000)" false))
    (:NewEnumerator1
      (Rendering|Material|SetMaterial _button 0 "/Game/Materials/Materials/Coins/MI_Coin_Green.MI_Coin_Green")
      (Rendering|Material|SetMaterial _sphere 0 "/Game/Materials/Materials/Glass/MI_FutigerGlass_Green.MI_FutigerGlass_Green")
      (Rendering|Components|Light|SetLightColor _pointlight "(R=0.250980,G=0.627451,B=0.258824,A=1.000000)" false))
    (:NewEnumerator2
      (Rendering|Material|SetMaterial _button 0 "/Game/Materials/Shaders/M_Coin.M_Coin")
      (Rendering|Material|SetMaterial _sphere 0 "/Game/Materials/Materials/Glass/FutigerGlass_Inst.FutigerGlass_Inst")
      (Rendering|Components|Light|SetLightColor _pointlight "(R=0.203922,G=0.447059,B=1.000000,A=1.000000)" false))
    (:NewEnumerator3
      (Rendering|Material|SetMaterial _button 0 "/Game/Materials/Materials/Coins/Mi_Coin_Yellow.Mi_Coin_Yellow")
      (Rendering|Material|SetMaterial _sphere 0 "/Game/Materials/Materials/Glass/MI_FutigerGlass_Yellow.MI_FutigerGlass_Yellow")
      (Rendering|Components|Light|SetLightColor _pointlight "(R=1.000000,G=0.823529,B=0.172549,A=1.000000)" false))
    (:NewEnumerator4
      (Rendering|Material|SetMaterial _button 0 "/Engine/VREditor/BasicMeshes/M_Floor_01.M_Floor_01")
      (Rendering|Material|SetMaterial _button 1 "/Game/Materials/Materials/MI_Mirror.MI_Mirror")
      (Rendering|Material|SetMaterial _sphere 0 "/Engine/VREditor/BasicMeshes/M_Floor_01.M_Floor_01"))))