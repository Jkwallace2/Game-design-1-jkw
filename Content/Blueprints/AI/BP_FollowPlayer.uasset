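; BP_FollowPlayer is an AI pawn that continually follows the player character.
; On BeginPlay it prints a count of actors tagged as test patrol points, which are not otherwise used, then starts the movement event.
; That event runs AI MoveTo toward the player with an acceptance radius, prints success or failure, and calls itself again after a short delay either way.
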(event Custom|move%20to
  (AI|AIMoveTo self "0, 0, 0" (Game|GetPlayerCharacter 0) 2e+02 false
    (:OnSuccess
      (Development|PrintString "Ai found player"))
    (:OnFail
      (Development|PrintString "Ai cant find player")))
  (Utilities|FlowControl|Delay 1.0)
  (CallFunction|Moveto))

(event EventBeginPlay
  (bind _outactors (Actor|GetAllActorsOfClasswithTag "/Script/Engine.Actor" "PatrollPointTest"))
  (Development|PrintString (Utilities|String|Append "there are" (Utilities|String|ToString(Integer) (Utilities|Array|Length _outactors)) "controll points"))
  (CallFunction|Moveto))

(fn ConstructionScript)