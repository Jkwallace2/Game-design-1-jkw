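; AI character that patrols the level between actors tagged PatrollPointTest.
; On BeginPlay it gathers and shuffles those points, then Patroll loops through AIMoveTo, advancing after success or failure and reshuffling after each full lap.
; Each leg gets a randomized walk speed.
; A gotoplayer event can move it to the player, but nothing here calls it and its follow-up MoveTo function is empty.
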(event Custom|Patroll
  ;[1 1 1] patrol
  (AI|AIMoveTo self (Transformation|GetActorLocation (Utilities|Array|Get(acopy) (stale EventBeginPlay _outactors) (Variables|Default|GetControllPointINdex))) 0 2e+02 false
    (:OnSuccess
      (Development|PrintString "Ai found player"))
    (:OnFail
      (Development|PrintString "Ai cant find player")))
  (bind _result (Math|Integer|IncrementInt (Variables|Default|GetControllPointINdex))
    (:%20%20
      (if (>= _result (Utilities|Array|Length (stale EventBeginPlay _outactors)))
        (Variables|Default|SetControllPointINdex 0)
        (Utilities|Array|Shuffle (stale EventBeginPlay _outactors))
        (else
          (Utilities|FlowControl|Delay 1.0)))
      (Variables|/Script/Engine.CharacterMovementComponent|SetMaxWalkSpeed (Variables|Character|GetCharacterMovement) (* (Math|Random|RandomIntegerinRange 8 25) 25.0))
      (CallFunction|Patroll))))

(event Custom|go%20to%20player
  ;[1 1 1] go to player
  (AI|AIMoveTo self "0, 0, 0" (Game|GetPlayerCharacter 0) 2e+02 false
    (:OnSuccess
      (Development|PrintString "Ai found player"))
    (:OnFail
      (Development|PrintString "Ai cant find player")))
  (Utilities|FlowControl|Delay 1.0)
  (CallFunction|Moveto))

(event EventBeginPlay
  (Variables|Default|SetControllPointINdex 0)
  (bind _outactors (Actor|GetAllActorsOfClasswithTag "/Script/Engine.Actor" "PatrollPointTest"))
  (Utilities|Array|Shuffle _outactors)
  (CallFunction|Patroll))

(fn ConstructionScript)

(fn Moveto)