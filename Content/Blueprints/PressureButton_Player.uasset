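; Player-triggered pressure button that activates a linked gate target or ball spawner.
; When the custom third-person character overlaps its Box, the button swaps to an activated material, then returns to walnut after a one-second delay.
; It activates the gate target if valid, otherwise the ball spawner, then prints a debug message that always names the gate target.
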(event OnComponentBeginOverlap(Box)
  (params (OverlappedComponent :type Primitive%20Component%20Object%20Reference) (OtherActor :type Actor%20Object%20Reference) (OtherComp :type Primitive%20Component%20Object%20Reference) (OtherBodyIndex :type Integer) (bFromSweep :type Boolean) (SweepResult :type Hit%20Result%20Structure%20%28by%20ref%29))
  (bind _target_ball_spawner (Variables|Default|GetTarget%20Ball%20Spawner))
  (bind _target_gate_target (Variables|Default|GetTarget%20Gate%20target))
  (Utilities|Casting|CastToBP_ThirdPersonCharacterCustom OtherActor) ; Did the player step on our platform?
  (CallFunction|Activate)
  (if (Utilities|IsValid _target_gate_target)
    (Default|Activate _target_gate_target)
    (Development|PrintString (Utilities|String|Append "sending data to " (Utilities|GetDisplayName _target_gate_target)) :!label _label)
    (elif (Utilities|IsValid _target_ball_spawner)
      (Default|Activate _target_ball_spawner)
      (goto _label))))

(event Custom|Activate
  (bind _button (Variables|Default|GetButton))
  (Rendering|Material|SetMaterial _button 0 "/Game/Materials/Materials/MI_PlatformActivated.MI_PlatformActivated") ; Change the color of the platform to "Activated"
  (Utilities|FlowControl|Delay 1.0)
  (Rendering|Material|SetMaterial _button 0 "/Game/StarterContent/Materials/M_Wood_Walnut.M_Wood_Walnut") ; Change the color of the platform to "Activated"
)

(event EventBeginPlay)

(event Collision|EventActorBeginOverlap
  (params (OtherActor :type Actor%20Object%20Reference)))

(event EventTick
  (params (DeltaSeconds :type Float%20%28single-precision%29)))

(fn ConstructionScript
  (Rendering|SetVisibility (Variables|Default|GetButton) (Variables|Default|GetVisible) false))