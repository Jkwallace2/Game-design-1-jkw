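; Teleporter actor that sends the custom third-person character from its Start trigger to its End point through that character's checkpoint functions.
; On overlap with Start, it writes End's world location into the character's TeleportLocation, calls TpCheckpoint, then calls LoadCheckpoint after a short delay.
; Only End's location feeds the target transform, not its rotation.
; Camera blend and field-of-view nodes remain in the graph unconnected and never run.
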(event OnComponentBeginOverlap(Start)
  (params (OverlappedComponent :type Primitive%20Component%20Object%20Reference) (OtherActor :type Actor%20Object%20Reference) (OtherComp :type Primitive%20Component%20Object%20Reference) (OtherBodyIndex :type Integer) (bFromSweep :type Boolean) (SweepResult :type Hit%20Result%20Structure%20%28by%20ref%29))
  (bind _asbp_third_person_character_custom (Utilities|Casting|CastToBP_ThirdPersonCharacterCustom OtherActor))
  (Variables|/Game/Blueprints/BP_ThirdPersonCharacterCustom.BP_ThirdPersonCharacterCustom_C|SetTeleport%20location _asbp_third_person_character_custom (Math|Conversions|ToTransform(Vector) (Transformation|GetWorldLocation (Variables|Default|GetEnd))))
  (Default|TpCheckpoint _asbp_third_person_character_custom)
  (Utilities|FlowControl|Delay 0.2)
  (Default|LoadCheckpoint _asbp_third_person_character_custom))

(event EventBeginPlay)

(event Collision|EventActorBeginOverlap
  (params (OtherActor :type Actor%20Object%20Reference)))

(event EventTick
  (params (DeltaSeconds :type Float%20%28single-precision%29)))

(fn ConstructionScript)